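; Flying book obstacle that moves through Mover components, either as a player-triggered platform or as a falling "Obstacle2Killer" trap.
; Normally it moves while the player overlaps it, reverses otherwise, and unpauses a flight sound while moving.
; The killer variant plays a warning on first overlap, speeds up its Mover, then drops after a timer with a cartoon fall sound.
; Reset re-arms the drop; Shake is an uncalled experiment.
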(event Custom|Drop
  ;[1 1 1] Drop Obstacle2killer
  (Variables|/Script/LastStandAwakening.Mover|SetIsTriggered (Actor|GetComponentbyClass "/Script/LastStandAwakening.Mover") true)
  (Audio|PlaySoundatLocation "/Game/Sounds/DroppingBook/cartoon-fall.cartoon-fall" (Transformation|GetActorLocation) "0, 0, 0" 1.0 1.0 0.0 0 0 0 0))

(event EventBeginPlay
  (Variables|Default|SetStartLocation (Transformation|GetActorLocation))
  ;[1 1 1] Spawn & Pause Slow Fly Sound
  (if (not (Actor|ActorHasTag "Obstacle2Killer"))
    (bind _returnvalue (Audio|SpawnSoundatLocation "/Game/Sounds/FlyingBook/SlowFlyingBook.SlowFlyingBook" (Transformation|GetActorLocation) "0, 0, 0" 1.0 1.0 0.0 0 0))
    (Class|AudioComponent|SetPaused _returnvalue true)))

(event EventTick
  (params (DeltaSeconds :type Float%20%28single-precision%29))
  ;[1 1 1] Branch For Killer, Otherwise connect Overlapping actor straight Next Branch
  (if (not (Components|ComponentHasTag (Variables|Default|GetTriggerBox) "Obstacle2Killer"))
    (Utilities|FlowControl|Sequence
      (:then_0
        (CallFunction|PlayPauseSlowFlyBookSound (stale EventBeginPlay _returnvalue)))
      (:then_1
        ;[1 1 1] Move When Triggered, Move Back When not Triggered
        (if (Collision|IsOverlappingActor (Game|Player|GetPlayerPawn 0) :!class /Script/Engine.Actor)
          (for _array_element (Actor|GetComponentsByClass "/Script/LastStandAwakening.Mover")
            (Variables|/Script/LastStandAwakening.Mover|SetIsTriggered _array_element true))
          (else
            (for _array_element_2 (Actor|GetComponentsByClass "/Script/LastStandAwakening.Mover")
              (Variables|/Script/LastStandAwakening.Mover|SetIsTriggered _array_element_2 false))))))))

(event Collision|EventActorBeginOverlap
  (params (OtherActor :type Actor%20Object%20Reference))
  ;[1 1 1] Drop Obstacle2killer
  (if (not (Variables|Default|GetIsDropped))
    (Variables|Default|SetIsDropped true)
    (if (Components|ComponentHasTag (Variables|Default|GetTriggerBox) "Obstacle2Killer")
      (Utilities|Time|SetTimerbyFunctionName 0 "Drop" 1.0)
      (Variables|/Script/LastStandAwakening.Mover|SetSpeed (Actor|GetComponentbyClass "/Script/LastStandAwakening.Mover") 1e+03)
      (Audio|PlaySoundatLocation "/Game/Sounds/DroppingBook/WatchYourFeet.WatchYourFeet" (Transformation|GetActorLocation) "0, 0, 0" 1.0 1.0 0.0 0 0 0 0))))

(fn ConstructionScript)

(fn Reset
  (Variables|Default|SetIsDropped false))

(fn PlayPauseSlowFlyBookSound
  (params (SlowFlySound :type Audio%20Component%20Object%20Reference))
  (if (Variables|/Script/LastStandAwakening.Mover|GetIsMooving (Actor|GetComponentbyClass "/Script/LastStandAwakening.Mover"))
    (Class|AudioComponent|SetPaused SlowFlySound false)
    (else
      (Class|AudioComponent|SetPaused SlowFlySound true))))

(fn Shake
  (Development|PrintString "Shaking")
  (bind _output_get (Variables|Default|SetShakingTime (+ (Variables|Default|GetShakingTime) (Utilities|Time|GetWorldDeltaSeconds))))
  (Transformation|SetActorLocation (Math|Interpolation|VInterpTo "0, 0, 0" (Math|Vector|MakeVector 0.0 0.0 0.0) 0.0 1.0) false false))