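; BP_TriggerBox_TopFlyingBook is a trigger that plays the Level 1 flying book opening cutscene when the player pawn first overlaps it.
; A DoOnce gate disables input, plays a look montage on BP_OrangeBoy, then creates and plays the level sequence.
; A delay matching the sequence's duration then restores input and stops the montage, rather than binding to the sequence's finished event.
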(event Collision|EventActorBeginOverlap
  (params (OtherActor :type Actor%20Object%20Reference))
  (bind _output_get (Variables|Default|SetOther%20Actor OtherActor))
  (if (== _output_get (Game|Player|GetPlayerPawn 0))
    (Utilities|FlowControl|DoOnce false
      (:Completed
        (Input|DisableInput _output_get 0)
        (bind _asbp_orange_boy (Utilities|Casting|CastToBP_OrangeBoy _output_get))
        (Animation|PlayAnimMontage _asbp_orange_boy "/Game/Blueprints/Characters/OrangeBoy/AnimationsOrangeBoy/AM_OpenningLook.AM_OpenningLook" 1.2 "None")
        (bind _outactor (Sequencer|Player|CreateLevelSequencePlayer "/Game/Cinemography/LS_Level1_FlyingBookOpeningScene.LS_Level1_FlyingBookOpeningScene"))
        (Sequencer|Player|Play (Variables|/Script/LevelSequence.LevelSequenceActor|GetSequencePlayer _outactor) :!class /Script/MovieScene.MovieSceneSequencePlayer)
        (Utilities|FlowControl|Delay (Class|TimeManagementBlueprintLibrary|ToSeconds(QualifiedFrameTime) (Media|MediaPlayer|GetDuration (Variables|/Script/LevelSequence.LevelSequenceActor|GetSequencePlayer _outactor))))
        (Input|EnableInput _asbp_orange_boy 0)
        (Animation|StopAnimMontage _asbp_orange_boy "/Game/Blueprints/Characters/OrangeBoy/AnimationsOrangeBoy/AM_OpenningLook.AM_OpenningLook")))))

(fn ConstructionScript)