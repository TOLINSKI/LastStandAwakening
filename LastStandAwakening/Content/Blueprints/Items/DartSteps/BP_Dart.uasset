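; BP_Dart is a dart item actor, filed under DartSteps, that rises vertically back to its starting position.
; BeginPlay stores the start location, then Reset drops the actor to world Z zero at that X/Y and switches Tick off.
; While ticking, MoveDartsZ eases it toward the stored height with VInterpTo and disables Tick within one unit.
; Nothing in this Blueprint re-enables Tick.
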(event EventBeginPlay
  (Variables|Default|SetStartLocation (Transformation|GetActorLocation))
  (CallFunction|Reset))

(event EventTick
  (params (DeltaSeconds :type Float%20%28single-precision%29))
  ;[0 0.1797 1] Move To Start Location (Up)
  (CallFunction|MoveDartsZ (Variables|Default|GetStartLocation)))

(fn ConstructionScript)

(fn MoveDartsZ
  (params (TargetLocation :type Vector))
  (bind _startlocation (Variables|Default|GetStartLocation))
  (Variables|Default|SetTargetLocation TargetLocation)
  (if (> (Math|Float|Absolute(Float) (- (.z (Transformation|GetActorLocation)) (.z (Variables|Default|GetTargetLocation)))) 1.0)
    (Transformation|SetActorLocation (Math|Interpolation|VInterpTo (Transformation|GetActorLocation) (Math|Vector|MakeVector (.x _startlocation) (.y _startlocation) (.z (Variables|Default|GetTargetLocation))) (Utilities|Time|GetWorldDeltaSeconds) 0.8) false true)
    (else
      (Actor|Tick|SetActorTickEnabled false))))

(fn Reset
  (bind _startlocation (Variables|Default|GetStartLocation))
  (Transformation|SetActorLocation (Math|Vector|MakeVector (.x _startlocation) (.y _startlocation) 0.0) false true)
  (Actor|Tick|SetActorTickEnabled false))