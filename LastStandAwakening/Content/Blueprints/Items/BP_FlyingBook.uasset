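; BP_FlyingBook is a flying book that moves while the player pawn overlaps it.
; Each tick sets IsTriggered on its Mover components from that overlap, so the book moves back when the player leaves.
; A slow-flying sound spawns paused at BeginPlay and plays only while the Mover reports movement.
; Tagging TriggerBox as Obstacle2Killer disables both the sound and the overlap-driven triggering.
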(event EventBeginPlay
  (Variables|Default|SetMover (Actor|GetComponentbyClass "/Script/LastStandAwakening.Mover"))
  (Variables|Default|SetStartLocation (Transformation|GetActorLocation))
  ;[1 1 1] Spawn & Pause Slow Fly Sound
  (if (not (Components|ComponentHasTag (Variables|Default|GetTriggerBox) "Obstacle2Killer"))
    (bind _returnvalue (Audio|SpawnSoundatLocation "/Game/Sounds/FlyingBook/SlowFlyingBook.SlowFlyingBook" (Transformation|GetActorLocation) "0, 0, 0" 1.0 1.0 0.0 0 0))
    (Class|AudioComponent|SetPaused _returnvalue true)))

(event EventTick
  (params (DeltaSeconds :type Float%20%28single-precision%29))
  (if (not (Components|ComponentHasTag (Variables|Default|GetTriggerBox) "Obstacle2Killer"))
    (Utilities|FlowControl|Sequence
      (:then_0
        (CallFunction|PlayPauseSlowFlyBookSound (stale EventBeginPlay _returnvalue)))
      (:then_1
        ;[1 1 1] Move When Triggered, Move Back When not Triggered
        (if (Collision|IsOverlappingActor (Game|Player|GetPlayerPawn 0) :!class /Script/Engine.Actor)
          (for _array_element (Actor|GetComponentsByClass "/Script/LastStandAwakening.Mover")
            (Variables|/Script/LastStandAwakening.Mover|SetIsTriggered _array_element true))
          (else
            (for _array_element_2 (Actor|GetComponentsByClass "/Script/LastStandAwakening.Mover")
              (Variables|/Script/LastStandAwakening.Mover|SetIsTriggered _array_element_2 false))))))))

(fn ConstructionScript)

(fn Reset
  (Variables|Default|SetIsDropped false))

(fn PlayPauseSlowFlyBookSound
  (params (SlowFlySound :type Audio%20Component%20Object%20Reference))
  (if (Variables|/Script/LastStandAwakening.Mover|GetIsMooving (Actor|GetComponentbyClass "/Script/LastStandAwakening.Mover"))
    (Class|AudioComponent|SetPaused SlowFlySound false)
    (else
      (Class|AudioComponent|SetPaused SlowFlySound true))))

(fn Shake)