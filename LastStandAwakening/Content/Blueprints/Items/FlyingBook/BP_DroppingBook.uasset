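; BP_DroppingBook is a one-shot falling book hazard that fires on its first actor overlap.
; The overlap sets IsDropped, then, if its TriggerBox is tagged Obstacle2Killer, sets Mover speed, starts Shaker and plays an earthquake sound.
; A timer calls Drop after a short delay, which stops the shake, triggers the Mover and plays a cartoon fall sound.
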(event Custom|Drop
  ;[1 1 1] Drop Obstacle2killer
  (Variables|/Script/LastStandAwakening.Shaker|SetbShake (Variables|Default|GetShaker) false)
  (Variables|/Script/LastStandAwakening.Mover|SetIsTriggered (Variables|Default|GetMover) true)
  (Audio|PlaySoundatLocation "/Game/Sounds/DroppingBook/cartoon-fall.cartoon-fall" (Transformation|GetActorLocation) "0, 0, 0" 1.0 1.0 0.0 0 0 0 0))

(event EventBeginPlay
  (|CallParentFunction) ; This node is disabled and will not be called.\nDrag off pins to build functionality.
)

(event EventTick
  (params (DeltaSeconds :type Float%20%28single-precision%29))
  (|CallParentFunction DeltaSeconds) ; This node is disabled and will not be called.\nDrag off pins to build functionality.
)

(event Collision|EventActorBeginOverlap
  (params (OtherActor :type Actor%20Object%20Reference))
  ;[1 1 1] Drop Obstacle2killer
  (if (not (Variables|Default|GetIsDropped))
    (Variables|Default|SetIsDropped true)
    (if (Components|ComponentHasTag (Variables|Default|GetTriggerBox) "Obstacle2Killer")
      (Utilities|Time|SetTimerbyFunctionName 0 "Drop" 1.0)
      (Utilities|FlowControl|Sequence
        (:then_0
          (Variables|/Script/LastStandAwakening.Mover|SetSpeed (Variables|Default|GetMover) 1e+03))
        (:then_1
          (Variables|/Script/LastStandAwakening.Shaker|SetbShake (Variables|Default|GetShaker) true))
        (:then_2
          (Audio|PlaySoundatLocation "/Game/Sounds/DroppingBook/SFX_EarthQuake.SFX_EarthQuake" (Transformation|GetActorLocation) "0, 0, 0" 1.0 1.0 0.0 0 0 0 0))))))

(fn ConstructionScript
  (|CallParentFunction))