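; BP_Weight is a weight item with a static mesh that can be returned to where it started.
; On BeginPlay it records its actor location and rotation.
; Its Reset function enables physics simulation on the mesh, then teleports the actor back to that stored transform without sweeping.
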(event EventBeginPlay
  (CallFunction|SetStartLocation&Rotation))

(event Collision|EventActorBeginOverlap
  (params (OtherActor :type Actor%20Object%20Reference)))

(event EventTick
  (params (DeltaSeconds :type Float%20%28single-precision%29)))

(fn ConstructionScript)

(fn Reset
  (Utilities|FlowControl|Sequence
    (:then_0
      (Physics|SetSimulatePhysics (Variables|Debug|GetStaticMeshComponent) true))
    (:then_1
      (Transformation|SetActorLocation (Variables|Default|GetStartLocation) false true)
      (Transformation|SetActorRotation (Variables|Default|GetStartRotation) true))))

(fn SetStartLocation&Rotation
  (Variables|Default|SetStartLocation (Transformation|GetActorLocation))
  (Variables|Default|SetStartRotation (Transformation|GetActorRotation)))