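; BP_RolyPoly is the roly-poly Blueprint that presents the game-won celebration through a widget component and sound.
; ShowGameWonWidget shows the widget, pauses the first AmbientSound actor's audio, then spawns and stores crowd-cheer and win-song sounds.
; HideWidgetAndSound hides the widget, stops both sounds and resumes the ambient audio, provided both stored sounds are valid.
; PlayStandUpSound is empty; its stand-up sound node is left unconnected.
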(event EventPlayStandUpSound
  ;[1 1 1] Play Sound When Standing Up
)

(event EventShowGameWonWidget
  (bind _returnvalue (Transformation|GetActorLocation))
  ;[1 1 1] Show\Hide WonGameWidget And Sounds
  (Default|Show (Variables|Default|GetWCBP_WinGameWidgetComponent))
  (bind _returnvalue_2 (Actor|GetActorOfClass "/Script/Engine.AmbientSound"))
  (bind _audiocomponent (Variables|/Script/Engine.AmbientSound|GetAudioComponent _returnvalue_2)
    (:then
      (Class|AudioComponent|SetPaused _audiocomponent true)
      (bind _returnvalue_3 (Audio|SpawnSoundatLocation "/Game/Sounds/GameWin/crowd-cheer.crowd-cheer" _returnvalue "0, 0, 0" 1.0 1.0 0.0 0 0))
      (Variables|Default|SetSoundCrowdCheer _returnvalue_3)
      (bind _returnvalue_4 (Audio|SpawnSoundatLocation "/Game/Sounds/GameWin/WinGameSongLong.WinGameSongLong" _returnvalue "0, 0, 0" 1.0 1.0 0.0 0 0))
      (Variables|Default|SetSoundHappyBday _returnvalue_4))
    (:else)))

(fn ConstructionScript)

(fn HideWidgetandSound
  (Default|Hide (Variables|Default|GetWCBP_WinGameWidgetComponent))
  (bind _soundcrowdcheer (Variables|Default|GetSoundCrowdCheer)
    (:then
      (Audio|Components|Audio|Stop _soundcrowdcheer)
      (bind _soundhappybday (Variables|Default|GetSoundHappyBday)
        (:then
          (Audio|Components|Audio|Stop _soundhappybday)
          (bind _returnvalue (Actor|GetActorOfClass "/Script/Engine.AmbientSound"))
          (Class|AudioComponent|SetPaused (Variables|/Script/Engine.AmbientSound|GetAudioComponent _returnvalue) false))
        (:else)))
    (:else)))